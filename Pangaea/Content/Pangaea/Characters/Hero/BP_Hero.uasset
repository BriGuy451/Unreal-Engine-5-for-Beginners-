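; Player hero Pawn with enhanced-input movement, attack and clamped spring-arm look, plus health shown on the HUD.
; AB_Hero's AnimState acts as the state machine, gating move, attack and damage and selecting hit or death, while Tick feeds it normalized speed.
; BeginPlay attaches a spawned sword to the hand, but its Weapon assignment is unwired.
; Death shows the lose screen, then destroys the hero and opens MainMenu after a delay.
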(event Input|EnhancedActionEvents|EnhancedInputActionAction_Attack
  (params (ActionValue :type Boolean) (ElapsedSeconds :type Float%20%28double-precision%29) (TriggeredSeconds :type Float%20%28double-precision%29) (InputAction :type Input%20Action%20Object%20Reference :default "/Game/Pangaea/Input/Actions/Action_Attack.Action_Attack"))
  (CallFunction|Attack))

(event Input|EnhancedActionEvents|EnhancedInputActionAction_Move
  (params (ActionValue :type Vector%202D%20Structure) (ElapsedSeconds :type Float%20%28double-precision%29) (TriggeredSeconds :type Float%20%28double-precision%29) (InputAction :type Input%20Action%20Object%20Reference :default "/Game/Pangaea/Input/Actions/Action_Move.Action_Move"))
  (bind (_x _y) (Math|Vector2D|BreakVector2D ActionValue))
  (CallFunction|MoveHero _x _y))

(event Input|EnhancedActionEvents|EnhancedInputActionAction_Hero_Look
  (params (ActionValue :type Vector%202D%20Structure) (ElapsedSeconds :type Float%20%28double-precision%29) (TriggeredSeconds :type Float%20%28double-precision%29) (InputAction :type Input%20Action%20Object%20Reference :default "/Game/Pangaea/Input/Actions/Action_Hero_Look.Action_Hero_Look"))
  (bind (_x _y) (Math|Vector2D|BreakVector2D ActionValue))
  (CallFunction|HeroLook _x _y))

(event EventBeginPlay
  (Utilities|FlowControl|Sequence
    (:then_0
      (bind _asab_hero (Utilities|Casting|CastToAB_Hero (Components|SkeletalMesh|GetAnimInstance (Variables|Character|GetMesh))))
      (Variables|/Game/Pangaea/Characters/Hero/AB_Hero.AB_Hero_C|SetAnimState _asab_hero 0))
    (:then_1
      (bind _returnvalue (Game|SpawnActorfromClass "/Game/Pangaea/Weapons/Sword/BP_Sword.BP_Sword_C" (Transformation|GetActorTransform) "AlwaysSpawn" "MultiplyWithRoot" 0 0))
      (Transformation|AttachComponentToComponent _returnvalue (Variables|Character|GetMesh) "hand_rSocket" "SnapToTarget" "SnapToTarget" "SnapToTarget" true))
    (:then_2
      (Variables|Default|SetHealth (Variables|Default|GetMaxHealth))
      (bind _foundwidgets (Widget|GetAllWidgetsOfClass "/Game/Pangaea/UI/HUD.HUD_C" true))
      (Default|UpdateHero (Utilities|Array|Get(acopy) _foundwidgets) self))))

(event Collision|EventActorBeginOverlap
  (params (OtherActor :type Actor%20Object%20Reference)))

(event EventTick
  (params (DeltaSeconds :type Float%20%28single-precision%29))
  (bind _returnvalue (Pawn|GetMovementComponent))
  ;[0.15 0.15 0.15 0.5] Sync Locomotion Animation
  (Variables|/Game/Pangaea/Characters/Hero/AB_Hero.AB_Hero_C|SetSpeed (CallFunction|GetAnimInst) (/ (Math|Vector|VectorLength (Class|NavMovementInterface|GetVelocityforNavMovement _returnvalue)) (Class|NavMovementInterface|GetMaxSpeedforNavMovement _returnvalue))))

(event Game|Damage|EventAnyDamage
  (params (Damage :type Float%20%28single-precision%29) (DamageType :type Damage%20Type%20Object%20Reference) (InstigatedBy :type Controller%20Object%20Reference) (DamageCauser :type Actor%20Object%20Reference))
  (Utilities|FlowControl|Sequence
    (:then_0
      ;[0.15 0.15 0.15 0.5] Take damage when ANimState is in locomotion and attack state
      (bind _asab_hero (Utilities|Casting|CastToAB_Hero (Components|SkeletalMesh|GetAnimInstance (Variables|Character|GetMesh))))
      (if (or (== (Variables|/Game/Pangaea/Characters/Hero/AB_Hero.AB_Hero_C|GetAnimState _asab_hero) 0) (== (Variables|/Game/Pangaea/Characters/Hero/AB_Hero.AB_Hero_C|GetAnimState _asab_hero) 1))
        (bind _output_get (Variables|Default|SetHealth (- (Variables|Default|GetHealth) Damage)))
        ;[0.15 0.15 0.15 0.5] Play the Hit animation if the hero is still alive, otherwise, play the Die animation
        (if (> _output_get 0.0)
          (Variables|/Game/Pangaea/Characters/Hero/AB_Hero.AB_Hero_C|SetAnimState _asab_hero 2)
          (else
            (Variables|/Game/Pangaea/Characters/Hero/AB_Hero.AB_Hero_C|SetAnimState _asab_hero 3)
            ;[0.15 0.15 0.15 0.5] Show You Lost!
            (bind _foundwidgets (Widget|GetAllWidgetsOfClass "/Game/Pangaea/UI/HUD.HUD_C" true))
            (Default|ShowWinLose (Utilities|Array|Get(acopy) _foundwidgets) false)
            (Utilities|FlowControl|Delay 5.0)
            (Actor|DestroyActor (Variables|Default|GetWeapon))
            (Actor|DestroyActor)
            (Game|OpenLevel(byName) "MainMenu")))))
    (:then_1
      ;[0.15 0.15 0.15 0.5] Update HUD hero info display
      (bind _foundwidgets_2 (Widget|GetAllWidgetsOfClass "/Game/Pangaea/UI/HUD.HUD_C" true))
      (Default|UpdateHero (Utilities|Array|Get(acopy) _foundwidgets_2) self))))

(fn ConstructionScript)

(fn GetAnimInst
  (bind _asab_hero (Utilities|Casting|CastToAB_Hero (Components|SkeletalMesh|GetAnimInstance (Variables|Character|GetMesh))))
  (return _asab_hero))

(fn Attack
  (bind _animinst (CallFunction|GetAnimInst))
  (if (== (Variables|/Game/Pangaea/Characters/Hero/AB_Hero.AB_Hero_C|GetAnimState _animinst) 0)
    (Variables|/Game/Pangaea/Characters/Hero/AB_Hero.AB_Hero_C|SetAnimState _animinst 1)))

(fn MoveHero
  (params (X%20Aixs :type Float%20%28double-precision%29) (Y%20Axis :type Float%20%28double-precision%29))
  ;[0.15 0.15 0.15 0.5] Check if Y Axis value is greater than 0. Only allows player to move forward
  (if (== (Variables|/Game/Pangaea/Characters/Hero/AB_Hero.AB_Hero_C|GetAnimState (CallFunction|GetAnimInst)) 0)
    ;[0.15 0.15 0.15 0.5] Move forward
    (Pawn|Input|AddControllerYawInput X%20Aixs)
    (Pawn|Input|AddMovementInput (Transformation|GetActorForwardVector) (+ (Math|Float|Absolute(Float) X%20Aixs) Y%20Axis) false)))

(fn HeroLook
  (params (X%20Axis :type Float%20%28double-precision%29) (Y%20Axis :type Float%20%28double-precision%29))
  (bind _springarm (Variables|Components|GetSpringArm))
  (bind _relativerotation (Variables|/Script/Engine.SceneComponent|GetRelativeRotation _springarm))
  (bind (_roll _pitch _yaw) (Math|Rotator|BreakRotator _relativerotation))
  ;[0.15 0.15 0.15 0.5] Rotating the camera view
  (Transformation|AddRelativeRotation (Variables|Components|GetSpringArm) (Math|Rotator|MakeRotator 0.0 X%20Axis Y%20Axis) false false)
  ;[0.15 0.15 0.15 0.5] Clamp the up/down the spring arm rotation within -30 and 30 degrees
  (Transformation|SetRelativeRotation _springarm (Math|Rotator|MakeRotator _roll (Math|Float|Clamp(Float) _pitch -3e+01 3e+01) _yaw) false false))