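; BP_WhileLoopFlow is a Blueprint that demonstrates while-loop flow control.
; On BeginPlay it sets X, then decrements it in a while loop, printing the new value each pass.
; When X reaches zero the loop exits and a final message is printed.
; The construction script is empty.
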(event EventBeginPlay
  (Variables|Default|SetX 20)
  (while (> (Variables|Default|GetX) 0)
    (bind _output_get (Variables|Default|SetX (- (Variables|Default|GetX) 1)))
    (Development|PrintString (Utilities|String|Append (Utilities|String|MakeLiteralString "x = ") (Utilities|String|ToString(Integer) _output_get))))
  (Development|PrintString "x is 0 now"))

(fn ConstructionScript)