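; BP_Mission runs a mission made of ordered objectives and handles the win condition, printing its goal at BeginPlay.
; Each Tick it scans the Objectives array, activates the first incomplete one and breaks, so objectives unlock in sequence.
; When none remain incomplete, a DoOnce shows the win screen on the HUD widget, then opens the MainMenu level after a delay.
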(event Custom|CustomEvent_Break
  (Utilities|Array|ForEachLoopwithBreak (Variables|Default|GetObjectives)) ; enters at Break
)

(event EventBeginPlay
  (Development|PrintString (Variables|Default|GetGoal) true true "(R=0.000000,G=0.660000,B=1.000000,A=1.000000)" 15.0))

(event EventTick
  (params (DeltaSeconds :type Float%20%28single-precision%29))
  (if (Variables|Default|GetIsCompleted)
    (Utilities|FlowControl|DoOnce false
      (:Completed
        (bind _foundwidgets (Widget|GetAllWidgetsOfClass "/Game/Pangaea/UI/HUD.HUD_C" true))
        (Default|ShowWinLose (Utilities|Array|Get(acopy) _foundwidgets) true)
        (Utilities|FlowControl|Delay 1e+01)
        (Game|OpenLevel(byName) "MainMenu")))
    (else
      (Variables|Default|SetIsCompleted true)
      (bind _array_element (Utilities|Array|ForEachLoopwithBreak (Variables|Default|GetObjectives))
        (:LoopBody
          (if (not (Variables|/Game/Pangaea/Mission/BP_Objective.BP_Objective_C|GetIsCompleted _array_element))
            (Variables|Default|SetIsCompleted false)
            (Variables|/Game/Pangaea/Mission/BP_Objective.BP_Objective_C|SetIsActive _array_element true)
            (CallFunction|CustomEventBreak)))))))

(fn ConstructionScript)