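; BP_Hammer is the melee weapon actor for the Warrok boss, dealing damage to actors it overlaps during attacks.
; On overlap it ignores its attach parent, which it casts to BP_Warrok.
; It applies a fixed damage amount only while the boss's anim instance AnimState matches one of two attack states, which are compared as hardcoded numbers.
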(event EventBeginPlay)

(event EventTick
  (params (DeltaSeconds :type Float%20%28single-precision%29)))

(event Collision|EventActorBeginOverlap
  (params (OtherActor :type Actor%20Object%20Reference))
  (bind _returnvalue (Actor|GetAttachParentActor))
  ;[0.15 0.15 0.15 0.5] Check if it is not Boss itself
  (if (!= OtherActor _returnvalue)
    (bind _asbp_warrok (Utilities|Casting|CastToBP_Warrok _returnvalue))
    ;[0.15 0.15 0.15 0.5] Check if is attacking
    (if (or (== (Variables|/Game/Pangaea/Characters/Warrok/AB_Warrok.AB_Warrok_C|GetAnimState (Default|GetAnimInst _asbp_warrok)) 11) (== (Variables|/Game/Pangaea/Characters/Warrok/AB_Warrok.AB_Warrok_C|GetAnimState (Default|GetAnimInst _asbp_warrok)) 12))
      (Game|Damage|ApplyDamage OtherActor 1e+02 0 self))))

(fn ConstructionScript)